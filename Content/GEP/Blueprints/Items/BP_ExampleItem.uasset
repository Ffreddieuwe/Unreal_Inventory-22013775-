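; Example world item that can be pushed and picked up, passing its class, icon, stack quantity and ID to the collector.
; On overlap with a BPI_Pickupable actor that is not another example item, it sends PickupMessage and destroys itself.
; PushItem applies a mass-independent velocity impulse to the mesh along player 0's facing direction, slightly offset from the item's origin.
; AddItemToStack, GetData and Pickup are stubs with empty or default results.
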(event Collision|EventActorBeginOverlap
  (params (OtherActor :type Actor%20Object%20Reference))
  (if (Utilities|DoesObjectImplementInterface OtherActor "/Game/GEP/Blueprints/Interfaces/BPI_Pickupable.BPI_Pickupable_C")
    (if (not (Utilities|ClassIsChildOf (Utilities|GetClass OtherActor) "BP_ExampleItem_C"))
      (Class|BPIPickupable|Pickup(Message) OtherActor (Variables|Default|GetItemClass) (Variables|Default|GetItemIcon) (Variables|Default|GetStackQuantity) (Variables|Default|GetItemID))
      (Actor|DestroyActor))))

(event EventPushItem
  (bind _returnvalue (Game|GetPlayerCharacter 0))
  (bind _returnvalue_2 (Transformation|GetActorRotation _returnvalue))
  (bind _returnvalue_3 (Math|Vector|GetForwardVector _returnvalue_2))
  (Class|PrimitiveComponent|AddVelocityChangeImpulseatLocation (Variables|Default|GetMesh) (* _returnvalue_3 2.5e+02) (+ (Transformation|GetActorLocation) (* _returnvalue_3 "10.000000,0.000000,0.000000")) "None"))

(fn ConstructionScript)

(fn AddItemtoStack
  (return))

(fn GetData
  (return 0 0 0 ""))

(fn Pickup
  (params (ItemClass :type Actor%20Class%20Reference) (ItemIcon :type Texture%202D%20Object%20Reference) (StackQuantity :type Integer) (ItemID :type String))
  (return))